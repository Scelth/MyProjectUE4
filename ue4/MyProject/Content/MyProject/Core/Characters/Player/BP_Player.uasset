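; BP_Player is the player Blueprint, adding a camera spring arm effect for sprinting.
; BeginPlay caches the spring arm's default length.
; OnStartSprint plays a timeline that lerps the arm length from that default to a sprint length, and OnStopSprint reverses the same timeline to ease it back.
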(event `self.ReceiveBeginPlay`
  (set `self.Default arm lenght` (`SpringArmComponent.TargetArmLength` (`self.SpringArmComponent`))))

(event `self.OnStartSprint`
  (bind (_direction _springarmtimeline) (`Timeline|Spring arm sprint timeline` :!label _label)
    (:`Update`
      (set `SpringArmComponent.TargetArmLength` (`KismetMathLibrary.Lerp` (`self.Default arm lenght`) (`self.Spring arm lenght`) _springarmtimeline) (`self.SpringArmComponent`)))))

(event `self.OnStopSprint`
  (goto _label :!via `Reverse`))

(fn `UserConstructionScript`)